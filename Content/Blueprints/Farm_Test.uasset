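; Clickable farm plot actor that plants, waters, harvests or deletes crops according to the tool equipped in BP_TopDownGameMode.
; The hand tool plants the selected crop on its own looping one-second timer, or spawns a Tomato_Cannon.
; Growth events swap meshes by elapsed time and pause when dry until the bucket resumes them.
; Sickle harvests add yield to game mode totals and free the plot, except apple trees, which regrow after a delay.
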(event `self.ReceiveBeginPlay`
  (bind _asbp_top_down_game_mode (cast `/Game/TopDown/Blueprints/BP_TopDownGameMode` (`GameplayStatics.GetGameMode`)))
  (set `self.Top Down Game Mode` _asbp_top_down_game_mode)
  (set `/Game/TopDown/Blueprints/BP_TopDownGameMode.Crop Type` "NewEnumerator4" (`self.Top Down Game Mode`))
  (`StaticMeshComponent.SetStaticMesh` (`self.replaceable actor`) null)
  (set `self.crop states` "NewEnumerator4"))

(event `grow wheat`
  (bind _output_get (set `self.wheat growing time` (+ (`self.wheat growing time`) 1)))
  (`KismetSystemLibrary.PrintString` (`KismetStringLibrary.Conv_IntToString` _output_get))
  (if (> _output_get 150)
    (if (< _output_get 300)
      (`StaticMeshComponent.SetStaticMesh` (`self.replaceable actor`) "/Game/assets/crop/wheat/between/wheat_bn.wheat_bn")
      (else
        (set `self.wheat growing time` 0)
        (`StaticMeshComponent.SetStaticMesh` (`self.replaceable actor`) "/Game/assets/crop/wheat/harvest/Wheat_3.Wheat_3")
        (set `self.crop states` "NewEnumerator2")
        (set `self.drying time` 0)
        (`KismetSystemLibrary.PrintString` "harvested")
        (`KismetSystemLibrary.K2_ClearAndInvalidateTimerHandle` (stale _returnvalue))))
    (elif (> _output_get (`self.drying time`))
      (`KismetSystemLibrary.PrintString` "crop is ready to be watered")
      (set `self.crop states` "NewEnumerator1")
      (`KismetSystemLibrary.K2_PauseTimerHandle` (stale _returnvalue)))))

(event `self.farm base.OnClicked`
  (params (TouchedComponent :type "PrimitiveComponent Object Reference") (ButtonPressed :type "Key Structure"))
  (bind _returnvalue_location (`KismetMathLibrary.BreakTransform` (`SceneComponent.K2_GetComponentToWorld` (`self.replaceable actor`))))
  (bind _crop_type (`/Game/TopDown/Blueprints/BP_TopDownGameMode.Crop Type` (`self.Top Down Game Mode`)))
  (bind _crop_type_2 (`/Game/TopDown/Blueprints/BP_TopDownGameMode.Crop Type` (`self.Top Down Game Mode`)))
  (bind _crop_type_3 (`/Game/TopDown/Blueprints/BP_TopDownGameMode.Crop Type` (`self.Top Down Game Mode`)))
  (bind _crop_type_4 (`/Game/TopDown/Blueprints/BP_TopDownGameMode.Crop Type` (`self.Top Down Game Mode`)))
  (bind _crop_type_5 (`/Game/TopDown/Blueprints/BP_TopDownGameMode.Crop Type` (`self.Top Down Game Mode`)))
  (bind _crop_type_6 (`/Game/TopDown/Blueprints/BP_TopDownGameMode.Crop Type` (`self.Top Down Game Mode`)))
  (if (`/Game/TopDown/Blueprints/BP_TopDownGameMode.is delete button equipped` (`self.Top Down Game Mode`))
    (`self.K2_DestroyActor`)
    (elif (`self.is growing a plant?`)
      (`|ExecutionSequence`
        (:`then_0`
          (if (`/Game/TopDown/Blueprints/BP_TopDownGameMode.is bucket equipped?` (`self.Top Down Game Mode`))
            (if (`|EnumEquality` (`self.crop states`) "NewEnumerator1")
              (`KismetSystemLibrary.PrintString` "crop is ready to be grown again")
              (set `self.crop states` "NewEnumerator0")
              (`|ExecutionSequence`
                (:`then_0`
                  (if (`|EnumEquality` (`self.currently growing crop`) "NewEnumerator0")
                    (`StaticMeshComponent.SetStaticMesh` (`self.replaceable actor`) "/Game/assets/crop/wheat/between/wheat_bn.wheat_bn")
                    (set `self.drying time` 1000)
                    (`KismetSystemLibrary.K2_UnPauseTimerHandle` (stale _returnvalue))
                    (`StaticMeshComponent.SetStaticMesh` (`self.replacable seeds`) null)))
                (:`then_1`
                  (if (`|EnumEquality` (`self.currently growing crop`) "NewEnumerator2")
                    (set `self.drying time` 1000)
                    ; carrot
                    (`KismetSystemLibrary.K2_UnPauseTimerHandle` (stale `self.farm base.OnClicked` _returnvalue_3))
                    (`StaticMeshComponent.SetStaticMesh` (`self.replaceable actor`) "/Game/assets/crop/carrot/Carrot_1.Carrot_1")
                    (`StaticMeshComponent.SetStaticMesh` (`self.replacable seeds`) null)))
                (:`then_2`
                  (if (`|EnumEquality` (`self.currently growing crop`) "NewEnumerator6")
                    (set `self.drying time` 1000)
                    ; tamhotar
                    (`KismetSystemLibrary.K2_UnPauseTimerHandle` (stale `self.farm base.OnClicked` _returnvalue_5))
                    (`StaticMeshComponent.SetStaticMesh` (`self.replaceable actor`) "/Game/assets/crop/tomato/Tomato_1.Tomato_1")
                    (`StaticMeshComponent.SetStaticMesh` (`self.replacable seeds`) null)))
                (:`then_3`
                  (if (`|EnumEquality` (`self.currently growing crop`) "NewEnumerator7")
                    (set `self.drying time` 1000)
                    ; berry
                    (`KismetSystemLibrary.K2_UnPauseTimerHandle` (stale `self.farm base.OnClicked` _returnvalue_6))
                    (`StaticMeshComponent.SetStaticMesh` (`self.replaceable actor`) "/Game/assets/crop/berry/Berry_1.Berry_1")
                    (`StaticMeshComponent.SetStaticMesh` (`self.replacable seeds`) null)))
                (:`then_4`
                  (if (`|EnumEquality` (`self.currently growing crop`) "NewEnumerator1")
                    (set `self.drying time` 1000)
                    ; apple
                    (`KismetSystemLibrary.K2_UnPauseTimerHandle` (stale `self.farm base.OnClicked` _returnvalue_2))
                    (`StaticMeshComponent.SetStaticMesh` (`self.replaceable actor`) "/Game/assets/crop/apple/AppleTree_2.AppleTree_2")))
                (:`then_5`
                  (if (`|EnumEquality` (`self.currently growing crop`) "NewEnumerator5")
                    (set `self.drying time` 1000)
                    (`StaticMeshComponent.SetStaticMesh` (`self.replacable seeds`) "/Game/assets/pumpkin/Pumpkin_1.Pumpkin_1")
                    (`KismetSystemLibrary.K2_UnPauseTimerHandle` (stale `self.farm base.OnClicked` _returnvalue_4))
                    (`StaticMeshComponent.SetStaticMesh` (`self.replaceable actor`) "/Game/assets/pumpkin/Pumpkin_1.Pumpkin_1"))))
              (else
                (`KismetSystemLibrary.PrintString` "crop not dried")))))
        (:`then_1`
          (if (`/Game/TopDown/Blueprints/BP_TopDownGameMode.is sickle equipped?` (`self.Top Down Game Mode`))
            (`self.harvest function`))))
      (elif (`/Game/TopDown/Blueprints/BP_TopDownGameMode.is hand key equipped?` (`self.Top Down Game Mode`))
        (`|ExecutionSequence`
          (:`then_0`
            (if (`|EnumEquality` _crop_type_6 "NewEnumerator0")
              (set `self.currently growing crop` "NewEnumerator0")
              (`KismetSystemLibrary.PrintString` (`|GetEnumeratorNameAsString` _crop_type_6))
              (set `self.is growing a plant?` true)
              (set `self.crop states` "NewEnumerator5")
              (`StaticMeshComponent.SetStaticMesh` (`self.replacable seeds`) "/Game/assets/seed/Wheat_seed.Wheat_seed")
              (bind _returnvalue (`KismetSystemLibrary.K2_SetTimerDelegate` (delegate `grow wheat`) 1.0 true))))
          (:`then_1`
            (if (`|EnumEquality` _crop_type_3 "NewEnumerator1")
              (set `self.currently growing crop` "NewEnumerator1")
              (set `self.health` 500.0)
              (`KismetSystemLibrary.PrintString` (`|GetEnumeratorNameAsString` _crop_type_3))
              (set `self.is growing a plant?` true)
              (set `self.crop states` "NewEnumerator5")
              (`StaticMeshComponent.SetStaticMesh` (`self.replaceable actor`) "/Game/assets/crop/apple/AppleTree_1.AppleTree_1")
              (bind _returnvalue_2 (`KismetSystemLibrary.K2_SetTimerDelegate` (delegate `Grow Apple`) 1.0 true))))
          (:`then_2`
            (if (`|EnumEquality` _crop_type "NewEnumerator2")
              (set `self.currently growing crop` "NewEnumerator2")
              (set `self.health` 80.0)
              (`KismetSystemLibrary.PrintString` (`|GetEnumeratorNameAsString` _crop_type))
              (set `self.is growing a plant?` true)
              (`StaticMeshComponent.SetStaticMesh` (`self.replacable seeds`) "/Game/assets/seed/Carrot_Seed.Carrot_Seed")
              (set `self.crop states` "NewEnumerator5")
              (bind _returnvalue_3 (`KismetSystemLibrary.K2_SetTimerDelegate` (delegate `Grow Carrot`) 1.0 true))))
          (:`then_3`
            (if (`|EnumEquality` (`/Game/TopDown/Blueprints/BP_TopDownGameMode.Crop Type` (`self.Top Down Game Mode`)) "NewEnumerator4")
              (`KismetSystemLibrary.PrintString` "select a plant to grow")))
          (:`then_4`
            (if (`|EnumEquality` _crop_type_5 "NewEnumerator5")
              (set `self.currently growing crop` "NewEnumerator5")
              (set `self.health` 200.0)
              (`KismetSystemLibrary.PrintString` (`|GetEnumeratorNameAsString` _crop_type_5))
              (set `self.is growing a plant?` true)
              (`StaticMeshComponent.SetStaticMesh` (`self.replacable seeds`) "/Game/assets/pumpkin/Pumpkin_Seed.Pumpkin_Seed")
              (set `self.crop states` "NewEnumerator5")
              (bind _returnvalue_4 (`KismetSystemLibrary.K2_SetTimerDelegate` (delegate `pumpkin grow`) 1.0 true))))
          (:`then_5`
            (if (`|EnumEquality` _crop_type_2 "NewEnumerator6")
              (set `self.currently growing crop` "NewEnumerator6")
              (set `self.health` 100.0)
              (`KismetSystemLibrary.PrintString` (`|GetEnumeratorNameAsString` _crop_type_2))
              (set `self.is growing a plant?` true)
              (`StaticMeshComponent.SetStaticMesh` (`self.replacable seeds`) "/Game/assets/seed/Tomato_Seed.Tomato_Seed")
              (set `self.crop states` "NewEnumerator5")
              (bind _returnvalue_5 (`KismetSystemLibrary.K2_SetTimerDelegate` (delegate `tomato grow`) 1.0 true))))
          (:`then_6`
            (if (`|EnumEquality` _crop_type_4 "NewEnumerator7")
              (set `self.currently growing crop` "NewEnumerator7")
              (set `self.health` 20.0)
              (`KismetSystemLibrary.PrintString` (`|GetEnumeratorNameAsString` _crop_type_4))
              (set `self.is growing a plant?` true)
              (`StaticMeshComponent.SetStaticMesh` (`self.replacable seeds`) "/Game/assets/seed/Berry_Seed.Berry_Seed")
              (set `self.crop states` "NewEnumerator5")
              (bind _returnvalue_6 (`KismetSystemLibrary.K2_SetTimerDelegate` (delegate `berry grow`) 1.0 true))))
          (:`then_7`
            (if (`|EnumEquality` (`/Game/TopDown/Blueprints/BP_TopDownGameMode.Crop Type` (`self.Top Down Game Mode`)) "NewEnumerator8")
              (`|SpawnActorFromClass` "/Game/Blueprints/Tomato_Cannon.Tomato_Cannon_C" (`KismetMathLibrary.MakeTransform` (+ _returnvalue_location (0.0 0.0 40.0))) "Undefined" "MultiplyWithRoot" null null))))
        (else
          (`KismetSystemLibrary.PrintString` "no bucket in hand"))))))

(event `Grow Apple`
  (bind _output_get (set `self.apple growing time` (+ (`self.apple growing time`) 1)))
  (`KismetSystemLibrary.PrintString` (`KismetStringLibrary.Conv_IntToString` _output_get))
  (if (> _output_get 10)
    (if (> _output_get 20)
      (set `self.apple growing time` 0)
      (set `self.crop states` "NewEnumerator2")
      (set `self.drying time` 0)
      (`KismetSystemLibrary.PrintString` "harvested")
      (`StaticMeshComponent.SetStaticMesh` (`self.replaceable actor`) "/Game/assets/crop/apple/AppleTree_5.AppleTree_5")
      (`KismetSystemLibrary.K2_ClearAndInvalidateTimerHandle` (stale `self.farm base.OnClicked` _returnvalue_2))
      (else
        (`StaticMeshComponent.SetStaticMesh` (`self.replaceable actor`) "/Game/assets/crop/apple/AppleTree_3.AppleTree_3")))
    (elif (> _output_get (`self.drying time`))
      (`KismetSystemLibrary.PrintString` "crop is ready to be watered")
      (set `self.crop states` "NewEnumerator1")
      (`KismetSystemLibrary.K2_PauseTimerHandle` (stale `self.farm base.OnClicked` _returnvalue_2)))))

(event `Grow apple tree`
  (`/Engine/EditorBlueprintResources/StandardMacros.DoOnce` false :!label _label
    (:`Completed`
      (set `self.crop states` "NewEnumerator0")
      (`StaticMeshComponent.SetStaticMesh` (`self.replaceable actor`) "/Game/assets/crop/apple/AppleTree_4.AppleTree_4")
      (`KismetSystemLibrary.Delay` 10.0)
      (`StaticMeshComponent.SetStaticMesh` (`self.replaceable actor`) "/Game/assets/crop/apple/AppleTree_5.AppleTree_5")
      (set `self.crop states` "NewEnumerator2")
      (goto _label :!via `Reset`))))

(event `Grow Carrot`
  (bind _output_get (set `self.carrot growing time` (+ (`self.carrot growing time`) 1)))
  (`KismetSystemLibrary.PrintString` (`KismetStringLibrary.Conv_IntToString` _output_get))
  (if (>= _output_get 600)
    (if (< _output_get 1200)
      (`StaticMeshComponent.SetStaticMesh` (`self.replaceable actor`) "/Game/assets/crop/carrot/Carrot_2.Carrot_2")
      (else
        (`StaticMeshComponent.SetStaticMesh` (`self.replaceable actor`) "/Game/assets/crop/carrot/Carrot_3.Carrot_3")
        (set `self.carrot growing time` 0)
        (set `self.crop states` "NewEnumerator2")
        (set `self.drying time` 0)
        (`KismetSystemLibrary.PrintString` "harvested")
        (`KismetSystemLibrary.K2_ClearAndInvalidateTimerHandle` (stale `self.farm base.OnClicked` _returnvalue_3))))
    (elif (> _output_get (`self.drying time`))
      (`KismetSystemLibrary.PrintString` "crop is ready to be watered")
      (set `self.crop states` "NewEnumerator1")
      (`KismetSystemLibrary.K2_PauseTimerHandle` (stale `self.farm base.OnClicked` _returnvalue_3)))))

(event `pumpkin grow`
  (bind _output_get (set `self.pumpkin growing time` (+ (`self.pumpkin growing time`) 1)))
  (`KismetSystemLibrary.PrintString` (`KismetStringLibrary.Conv_IntToString` _output_get))
  (if (> _output_get 600)
    (if (> _output_get 1200)
      (set `self.pumpkin growing time` 0)
      (set `self.crop states` "NewEnumerator2")
      (set `self.drying time` 5)
      (`StaticMeshComponent.SetStaticMesh` (`self.replaceable actor`) "/Game/assets/pumpkin/Pumpkin_3.Pumpkin_3")
      (`KismetSystemLibrary.PrintString` "harvested")
      (`KismetSystemLibrary.K2_ClearAndInvalidateTimerHandle` (stale `self.farm base.OnClicked` _returnvalue_4))
      (else
        (`StaticMeshComponent.SetStaticMesh` (`self.replaceable actor`) "/Game/assets/pumpkin/Pumpkin_2.Pumpkin_2")))
    (elif (> _output_get (`self.drying time`))
      (`KismetSystemLibrary.PrintString` "crop is ready to be watered")
      (set `self.crop states` "NewEnumerator1")
      (`KismetSystemLibrary.K2_PauseTimerHandle` (stale `self.farm base.OnClicked` _returnvalue_4)))))

(event `tomato grow`
  (bind _output_get (set `self.tomato growing time` (+ (`self.tomato growing time`) 1)))
  (`KismetSystemLibrary.PrintString` (`KismetStringLibrary.Conv_IntToString` _output_get))
  (if (> _output_get 600)
    (if (< _output_get 1200)
      (`StaticMeshComponent.SetStaticMesh` (`self.replaceable actor`) "/Game/assets/crop/tomato/Tomato_2.Tomato_2")
      (else
        (set `self.tomato growing time` 0)
        (set `self.crop states` "NewEnumerator2")
        (`StaticMeshComponent.SetStaticMesh` (`self.replaceable actor`) "/Game/assets/crop/tomato/Tomato_3.Tomato_3")
        (set `self.drying time` 0)
        (`KismetSystemLibrary.PrintString` "harvested")
        (`KismetSystemLibrary.K2_ClearAndInvalidateTimerHandle` (stale `self.farm base.OnClicked` _returnvalue_5))))
    (elif (> _output_get (`self.drying time`))
      (`KismetSystemLibrary.PrintString` "crop is ready to be watered")
      (set `self.crop states` "NewEnumerator1")
      (`StaticMeshComponent.SetStaticMesh` (`self.replaceable actor`) null)
      (`KismetSystemLibrary.K2_PauseTimerHandle` (stale `self.farm base.OnClicked` _returnvalue_5)))))

(event `berry grow`
  (bind _output_get (set `self.berry growing time` (+ (`self.berry growing time`) 1)))
  (`KismetSystemLibrary.PrintString` (`KismetStringLibrary.Conv_IntToString` _output_get))
  (if (> _output_get 300)
    (if (< _output_get 600)
      (`StaticMeshComponent.SetStaticMesh` (`self.replaceable actor`) "/Game/assets/crop/berry/Berry_2.Berry_2")
      (else
        (set `self.berry growing time` 0)
        (set `self.crop states` "NewEnumerator2")
        (`StaticMeshComponent.SetStaticMesh` (`self.replaceable actor`) "/Game/assets/crop/berry/Berry_3.Berry_3")
        (set `self.drying time` 0)
        (`KismetSystemLibrary.PrintString` "harvested")
        (`KismetSystemLibrary.K2_ClearAndInvalidateTimerHandle` (stale `self.farm base.OnClicked` _returnvalue_6))))
    (elif (> _output_get (`self.drying time`))
      (`KismetSystemLibrary.PrintString` "crop is ready to be watered")
      (`StaticMeshComponent.SetStaticMesh` (`self.replaceable actor`) null)
      (set `self.crop states` "NewEnumerator1")
      (`KismetSystemLibrary.K2_PauseTimerHandle` (stale `self.farm base.OnClicked` _returnvalue_6)))))

(fn `harvest function`
  (bind _top_down_game_mode (`self.Top Down Game Mode`))
  (bind _top_down_game_mode_2 (`self.Top Down Game Mode`))
  (bind _top_down_game_mode_3 (`self.Top Down Game Mode`))
  (bind _top_down_game_mode_4 (`self.Top Down Game Mode`))
  (bind _top_down_game_mode_5 (`self.Top Down Game Mode`))
  (bind _top_down_game_mode_6 (`self.Top Down Game Mode`))
  (if (`|EnumEquality` (`self.crop states`) "NewEnumerator2")
    (`|ExecutionSequence`
      (:`then_0`
        (if (`|EnumEquality` (`self.currently growing crop`) "NewEnumerator1")
          (bind _output_get (set `/Game/TopDown/Blueprints/BP_TopDownGameMode.apple amount` (+ (`/Game/TopDown/Blueprints/BP_TopDownGameMode.apple amount` _top_down_game_mode) 14) _top_down_game_mode))
          (`KismetSystemLibrary.PrintString` (`KismetStringLibrary.Conv_IntToString` _output_get))
          (`self.Grow apple tree`)))
      (:`then_1`
        (if (`|EnumEquality` (`self.currently growing crop`) "NewEnumerator7")
          (set `/Game/TopDown/Blueprints/BP_TopDownGameMode.berry amount` (+ (`/Game/TopDown/Blueprints/BP_TopDownGameMode.berry amount` _top_down_game_mode_5) 4) _top_down_game_mode_5)
          (`StaticMeshComponent.SetStaticMesh` (`self.replaceable actor`) null)
          (`KismetSystemLibrary.PrintString` "crop produced" :!label _label)
          (set `self.is growing a plant?` false)))
      (:`then_2`
        (if (`|EnumEquality` (`self.currently growing crop`) "NewEnumerator6")
          (set `/Game/TopDown/Blueprints/BP_TopDownGameMode.tomato amount` (+ (`/Game/TopDown/Blueprints/BP_TopDownGameMode.tomato amount` _top_down_game_mode_2) 3) _top_down_game_mode_2)
          (`StaticMeshComponent.SetStaticMesh` (`self.replaceable actor`) null :!label _label_2)
          (goto _label)))
      (:`then_3`
        (if (`|EnumEquality` (`self.currently growing crop`) "NewEnumerator5")
          (set `/Game/TopDown/Blueprints/BP_TopDownGameMode.pumpkin amount` (+ (`/Game/TopDown/Blueprints/BP_TopDownGameMode.pumpkin amount` _top_down_game_mode_3) 1) _top_down_game_mode_3)
          (`StaticMeshComponent.SetStaticMesh` (`self.replaceable actor`) null)
          (goto _label_2)))
      (:`then_4`
        (if (`|EnumEquality` (`self.currently growing crop`) "NewEnumerator2")
          (set `/Game/TopDown/Blueprints/BP_TopDownGameMode.carrot amount` (+ (`/Game/TopDown/Blueprints/BP_TopDownGameMode.carrot amount` _top_down_game_mode_4) 5) _top_down_game_mode_4)
          (`StaticMeshComponent.SetStaticMesh` (`self.replaceable actor`) null)
          (goto _label)))
      (:`then_5`
        (if (`|EnumEquality` (`self.currently growing crop`) "NewEnumerator0")
          (set `/Game/TopDown/Blueprints/BP_TopDownGameMode.wheat amount` (+ (`/Game/TopDown/Blueprints/BP_TopDownGameMode.wheat amount` _top_down_game_mode_6) 10) _top_down_game_mode_6)
          (`StaticMeshComponent.SetStaticMesh` (`self.replaceable actor`) null)
          (goto _label))))))

(fn `regrow timer`)

(fn `UserConstructionScript`)

(fn `wheat growth`)