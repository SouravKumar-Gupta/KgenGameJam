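; Clickable sphere actor that acts as a build spot for placing a test farm in the top-down game.
; On BeginPlay it caches the BP_TopDownGameMode, which holds the hand-key equipped flag and Currency.
; Clicking the sphere with the key equipped and enough currency deducts the cost and spawns Farm_Test at its X/Y and a fixed height.
; Debug prints report placement, insufficient money or a missing key selection.
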(event `self.ReceiveBeginPlay`
  (bind _asbp_top_down_game_mode (cast `/Game/TopDown/Blueprints/BP_TopDownGameMode` (`GameplayStatics.GetGameMode`)))
  (set `self.As BP Top Down Game Mode` _asbp_top_down_game_mode))

(event `self.Sphere.OnClicked`
  (params (TouchedComponent :type "PrimitiveComponent Object Reference") (ButtonPressed :type "Key Structure"))
  (bind _as_bp_top_down_game_mode (`self.As BP Top Down Game Mode`))
  (bind _returnvalue (`SceneComponent.K2_GetComponentToWorld` (`self.Sphere`)))
  (bind _currency (`/Game/TopDown/Blueprints/BP_TopDownGameMode.currency` _as_bp_top_down_game_mode))
  (if (`/Game/TopDown/Blueprints/BP_TopDownGameMode.is hand key equipped?` (`self.As BP Top Down Game Mode`))
    (`KismetSystemLibrary.PrintString` "a farm can be placed")
    (if (> _currency 10)
      (set `/Game/TopDown/Blueprints/BP_TopDownGameMode.currency` (- _currency 10) _as_bp_top_down_game_mode)
      (`|SpawnActorFromClass` "/Game/Blueprints/Farm_Test.Farm_Test_C" (`KismetMathLibrary.MakeTransform` (`KismetMathLibrary.MakeVector` (.x (.location _returnvalue)) (.y (.location _returnvalue)) 25.0)) "Undefined" "MultiplyWithRoot" null null)
      (else
        (`KismetSystemLibrary.PrintString` "get more money")))
    (else
      (`KismetSystemLibrary.PrintString` "select the farm key"))))

(fn `UserConstructionScript`)