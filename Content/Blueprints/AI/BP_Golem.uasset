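; Golem enemy AI that advances toward the MainTree, attacking fences, farms and the tree.
; Tick faces the tree, line-traces forward past other enemies, and uses hit tags to pick an AIMoveTo and attack.
; Attacks loop a montage, draining target health; fences leave broken versions, while destroyed crops can kill, slow or damage the golem by game-mode CropType.
; Tick also creates a new health bar widget each frame without displaying it.
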(event `self.ReceiveTick`
  (params (DeltaSeconds :type "Float (single-precision)"))
  (bind _scene (`self.Scene`))
  (bind _returnvalue (`SceneComponent.K2_GetComponentLocation` _scene))
  (`|ExecutionSequence`
    (:`then_0`
      (bind _returnvalue_2 (`GameplayStatics.GetActorOfClass` "/Game/Blueprints/MainTree.MainTree_C"))
      (bind (_returnvalue_roll _returnvalue_pitch _returnvalue_yaw) (`KismetMathLibrary.BreakRotator` (`KismetMathLibrary.FindLookAtRotation` (`self.K2_GetActorLocation`) (`self.K2_GetActorLocation` _returnvalue_2))))
      (`self.K2_SetActorRotation` (`KismetMathLibrary.MakeRotator` 0.0 0.0 _returnvalue_yaw))
      (if (not (`self.reached?`))
        (bind _outactors (`GameplayStatics.GetAllActorsOfClass` "/Game/Blueprints/AI/BP_EnemyBase.BP_EnemyBase_C"))
        (bind (_outhit _returnvalue_3) (`KismetSystemLibrary.LineTraceSingle` _returnvalue (+ _returnvalue (* (`KismetMathLibrary.GetForwardVector` (`SceneComponent.K2_GetComponentRotation` _scene)) 1000.0)) "TraceTypeQuery2" false _outactors "ForOneFrame" true (struct :`R` 1.0 :`A` 1.0) (struct :`G` 1.0 :`A` 1.0) 1.0))
        (if _returnvalue_3
          (bind (_bblockinghit _binitialoverlap _time _distance _location _impactpoint _normal _impactnormal _physmat _hitactor) (`GameplayStatics.BreakHitResult` _outhit))
          (if (`self.ActorHasTag` _hitactor "wall")
            (bind _output_get (set `self.hit location` _location))
            (set `self.hit` _hitactor)
            (`self.Move to wall` _output_get)
            (elif (`self.ActorHasTag` _hitactor "farm")
              (set `self.hit` _hitactor)
              (bind _output_get_2 (set `self.hit location` _location))
              (`self.Move to Farm` _output_get_2)
              (elif (`self.ActorHasTag` _hitactor "ped")
                (set `self.hit` _hitactor)
                (bind _output_get_3 (set `self.hit location` _location))
                (`self.Move to Tree` _output_get_3)))))))
    (:`then_1`
      (bind _returnvalue_4 (`|CreateWidget` "/Game/Blueprints/WB_EnemyHealthBar.WB_EnemyHealthBar_C"))
      (`ProgressBar.SetPercent` (`/Game/Blueprints/WB_EnemyHealthBar.healthbar` _returnvalue_4) (`KismetMathLibrary.FClamp` (`KismetMathLibrary.Conv_IntToDouble` (/ (`self.health`) 30)) 0.0 1.0)))))

(event `self.ReceiveBeginPlay`
  (`|ExecutionSequence`
    (:`then_0`
      (set `self.reached?` false))
    (:`then_1`
      (bind _asbp_top_down_game_mode (cast `/Game/TopDown/Blueprints/BP_TopDownGameMode` (`GameplayStatics.GetGameMode`)))
      (set `self.asTop Down Game Mode` _asbp_top_down_game_mode)
      (set `self.health` 50))))

(event `Move to wall`
  (params (Destination :type "Vector Structure"))
  (`|AIMoveTo` self Destination null 150.0
    (:`OnSuccess`
      (`/Engine/EditorBlueprintResources/StandardMacros.IsValid` (`self.hit`)
        (:`Is Valid`
          (set `self.reached?` true)
          (if (`self.ActorHasTag` (`self.hit`) "wall")
            (`self.Wall Attack`)))))))

(event `Wall Attack`
  (if (`self.reached?`)
    (`|ExecutionSequence`
      (:`then_0`
        (bind _asbp_top_fence (cast `/Game/Blueprints/Fences/BP_TopFence` (`self.hit`) :!label _label))
        (`|PlayMontage` (`self.Mesh`) "/Game/assets/enemy3/GolemMesh_Anim_Attack02_Montage.GolemMesh_Anim_Attack02_Montage"
          (:`OnCompleted`
            (bind _output_get (set `/Game/Blueprints/Fences/BP_TopFence.Health` (- (`/Game/Blueprints/Fences/BP_TopFence.Health` _asbp_top_fence) 1.0) _asbp_top_fence))
            (if (> _output_get 0.0)
              (goto _label)
              (else
                (`self.K2_DestroyActor` _asbp_top_fence)
                (`self.StopAnimMontage` "/Game/assets/enemy3/GolemMesh_Anim_Attack02_Montage.GolemMesh_Anim_Attack02_Montage")
                (`|SpawnActorFromClass` "/Game/Blueprints/Fences/BP_BrokenTopFence.BP_BrokenTopFence_C" (`KismetMathLibrary.MakeTransform` (`self.hit location`)) "Undefined" "MultiplyWithRoot" null null)
                (set `self.reached?` false))))))
      (:`then_1`
        (bind _asbp_left_fence (cast `/Game/Blueprints/Fences/BP_LeftFence` (`self.hit`) :!label _label_2))
        (`|PlayMontage` (`self.Mesh`) "/Game/assets/enemy3/GolemMesh_Anim_Attack02_Montage.GolemMesh_Anim_Attack02_Montage"
          (:`OnCompleted`
            (bind _output_get_2 (set `/Game/Blueprints/Fences/BP_LeftFence.Health` (- (`/Game/Blueprints/Fences/BP_LeftFence.Health` _asbp_left_fence) 1.0) _asbp_left_fence))
            (if (> _output_get_2 0.0)
              (goto _label_2)
              (else
                (`self.K2_DestroyActor` (`self.hit`))
                (`self.StopAnimMontage` "/Game/assets/enemy3/GolemMesh_Anim_Attack02_Montage.GolemMesh_Anim_Attack02_Montage")
                (`|SpawnActorFromClass` "/Game/Blueprints/Fences/BP_BrokenLeftFence.BP_BrokenLeftFence_C" (`KismetMathLibrary.MakeTransform` (`self.hit location`)) "Undefined" "MultiplyWithRoot" null null)
                (set `self.reached?` false)))))))))

(event `Move to Farm`
  (params (Destination :type "Vector Structure"))
  (bind _hit (`self.hit`))
  (`|AIMoveTo` self Destination null 100.0
    (:`OnSuccess`
      (`/Engine/EditorBlueprintResources/StandardMacros.IsValid` _hit
        (:`Is Valid`
          (if (`self.ActorHasTag` _hit "farm")
            (`self.Attack Farm`)
            (set `self.reached?` true)))))))

(event `Attack Farm`
  (bind _charactermovement (`self.CharacterMovement`))
  (bind _crop_type (`/Game/TopDown/Blueprints/BP_TopDownGameMode.Crop Type` (`self.asTop Down Game Mode`)))
  (if (`self.reached?`)
    (bind _asfarm_test (cast `/Game/Blueprints/Farm_Test` (`self.hit`) :!label _label_3))
    (`|PlayMontage` (`self.Mesh`) "/Game/assets/enemy3/GolemMesh_Anim_Attack02_Montage.GolemMesh_Anim_Attack02_Montage"
      (:`OnCompleted`
        (bind _output_get (set `/Game/Blueprints/Farm_Test.health` (- (`/Game/Blueprints/Farm_Test.health` _asfarm_test) 1.0) _asfarm_test))
        (if (> _output_get 0.0)
          (goto _label_3)
          (elif (`|EnumEquality` _crop_type "NewEnumerator7")
            (`self.K2_DestroyActor`)
            (else
              (if (`|EnumEquality` _crop_type "NewEnumerator5")
                (`self.K2_DestroyActor` (`self.hit`))
                (set `CharacterMovementComponent.MaxWalkSpeed` 5.0 _charactermovement)
                (`KismetSystemLibrary.Delay` 5.0)
                (set `CharacterMovementComponent.MaxWalkSpeed` 50.0 _charactermovement)
                (elif (`|EnumEquality` (`/Game/TopDown/Blueprints/BP_TopDownGameMode.Crop Type` (`self.asTop Down Game Mode`)) "NewEnumerator6")
                  (`self.K2_DestroyActor` (`self.hit`))
                  (set `self.health` (- (`self.health`) 10))
                  (set `CharacterMovementComponent.MaxWalkSpeed` 5.0 (`self.CharacterMovement`))
                  (`KismetSystemLibrary.Delay` 5.0)
                  (set `CharacterMovementComponent.MaxWalkSpeed` 50.0 (`self.CharacterMovement`))
                  (else
                    (`self.K2_DestroyActor` (`self.Hit`)))))
              (`self.StopAnimMontage` "/Game/assets/enemy3/GolemMesh_Anim_Attack02_Montage.GolemMesh_Anim_Attack02_Montage")
              (set `self.reached?` false))))))))

(event `Move to Tree`
  (params (Destination :type "Vector Structure"))
  (bind _hit (`self.hit`))
  (`|AIMoveTo` self Destination null 100.0
    (:`OnSuccess`
      (`/Engine/EditorBlueprintResources/StandardMacros.IsValid` _hit
        (:`Is Valid`
          (if (`self.ActorHasTag` _hit "ped")
            (`/Engine/EditorBlueprintResources/StandardMacros.DoOnce` false
              (:`Completed`
                (`self.Attack Tree`)
                (set `self.reached?` true)))))))))

(event `Attack Tree`
  (bind _asmain_tree (cast `/Game/Blueprints/MainTree` (`self.hit`) :!label _label_4))
  (`|PlayMontage` (`self.Mesh`) "/Game/assets/enemy3/GolemMesh_Anim_Attack02_Montage.GolemMesh_Anim_Attack02_Montage"
    (:`OnCompleted`
      (bind _output_get (set `/Game/Blueprints/MainTree.Tree Health` (- (`/Game/Blueprints/MainTree.Tree Health` _asmain_tree) 1.0) _asmain_tree))
      (if (> _output_get 0.0)
        (goto _label_4)
        (else
          (`self.K2_DestroyActor` (`self.hit`))
          (set `self.reached?` false))))))

(fn `UserConstructionScript`
  (`parent.UserConstructionScript`))