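; GridManager is an actor Blueprint that lays out a square grid of Sphere actors when play begins.
; BeginPlay calls AddGrid, whose nested loops spawn one Sphere per cell across Gridsize rows and columns.
; Each world position comes from the loop indices scaled by WorldGridSize and shifted by WorldOffset, plus a fixed nudge in X and Y and a slight drop in Z, independent of the manager's own location.
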(event `add grid`
  (bind _world_grid_size (`self.world grid size`))
  (bind _world_offset (`self.world offset`))
  (for _index (range (`self.gridsize`))
    (for _index_2 (range (`self.gridsize`))
      (bind (_returnvalue_x _returnvalue_y _returnvalue_z) (`KismetMathLibrary.BreakVector` (`KismetMathLibrary.MakeVector` (- (* _index_2 _world_grid_size) _world_offset) (- (* _world_grid_size _index) _world_offset))))
      (`|SpawnActorFromClass` "/Game/Blueprints/sphere.sphere_C" (`KismetMathLibrary.MakeTransform` (`KismetMathLibrary.MakeVector` (+ _returnvalue_x 50.0) (+ _returnvalue_y 50.0) (- _returnvalue_z 20.0))) "Undefined" "MultiplyWithRoot" null null))))

(event `self.ReceiveBeginPlay`
  (`self.add grid`))

(fn `UserConstructionScript`)