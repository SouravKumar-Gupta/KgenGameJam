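; MainTree is a tree actor that earns currency for the game mode and periodically spawns coins nearby.
; BeginPlay caches the top-down game mode, sets tree health and creates a player widget without adding it to the viewport.
; Tick uses delays to spawn Coins at random offsets and feed a looping currency increment.
; Logic that repeatedly damages and destroys overlapping enemies exists but is disconnected, so the sphere overlap does nothing.
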(event `self.ReceiveBeginPlay`
  (`|ExecutionSequence`
    (:`then_0`
      (bind _asbp_top_down_game_mode (cast `/Game/TopDown/Blueprints/BP_TopDownGameMode` (`GameplayStatics.GetGameMode`)))
      (set `self.As BP Top Down Game Mode` _asbp_top_down_game_mode)
      (set `self.Tree Health` 100.0))
    (:`then_1`
      (bind _returnvalue (`|CreateWidget` "/Game/Blueprints/wb_player.wb_player_C"))
      (set `self.ui` _returnvalue))))

(event `self.ReceiveTick`
  (params (DeltaSeconds :type "Float (single-precision)"))
  (bind (_returnvalue_x _returnvalue_y _returnvalue_z) (`KismetMathLibrary.BreakVector` (`self.K2_GetActorLocation`)))
  (`|ExecutionSequence`
    (:`then_0`
      (`KismetSystemLibrary.Delay` 35.0)
      (`|SpawnActorFromClass` "/Game/Blueprints/Coin.Coin_C" (`KismetMathLibrary.MakeTransform` (`KismetMathLibrary.MakeVector` (+ _returnvalue_x (`KismetMathLibrary.RandomFloatInRange` -250.0 -500.0)) (+ _returnvalue_y (`KismetMathLibrary.RandomFloatInRange` (`KismetMathLibrary.RandomFloatInRange` -100.0) (`KismetMathLibrary.RandomFloatInRange` 0.0 100.0))) (+ _returnvalue_z 200.0))) "AlwaysSpawn" "MultiplyWithRoot" null null)
      (`/Engine/EditorBlueprintResources/StandardMacros.IncrementInt` (`/Game/TopDown/Blueprints/BP_TopDownGameMode.currency` (`self.As BP Top Down Game Mode`)) :!label _label
        (:`  `
          (`KismetSystemLibrary.Delay` 25.0)
          (goto _label))))))

(event `self.Sphere.OnComponentBeginOverlap`
  (params (OverlappedComponent :type "PrimitiveComponent Object Reference") (OtherActor :type "Actor Object Reference") (OtherComp :type "PrimitiveComponent Object Reference") (OtherBodyIndex :type Integer) (bFromSweep :type Boolean) (SweepResult :type "HitResult Structure (by ref)")))

(fn `UserConstructionScript`)