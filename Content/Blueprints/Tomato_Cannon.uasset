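; Tomato cannon tower that attacks BP_EnemyBase actors entering its sphere while it has ammo, otherwise printing "get more ammo".
; Each hit directly decrements enemy Health, destroying it at zero, and spawns a TomatoProjectile from AttackPoint aimed at the line trace's end.
; Delay-driven loops repeat damage and firing without rechecking overlap; the firing loop also skips the ammo check.
; CurrentAmmo is never decremented here.
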(event `self.Sphere.OnComponentBeginOverlap`
  (params (OverlappedComponent :type "PrimitiveComponent Object Reference") (OtherActor :type "Actor Object Reference") (OtherComp :type "PrimitiveComponent Object Reference") (OtherBodyIndex :type Integer) (bFromSweep :type Boolean) (SweepResult :type "HitResult Structure (by ref)"))
  (bind _returnvalue (`SceneComponent.K2_GetComponentLocation` (`self.attack point`)))
  (if (> (`self.current ammo`) 0) :!label _label
    (bind _asbp_enemy_base (cast `/Game/Blueprints/AI/BP_EnemyBase` OtherActor :!label _label_2))
    (`/Engine/EditorBlueprintResources/StandardMacros.IsValid` _asbp_enemy_base
      (:`Is Valid`
        (bind _outhit (`KismetSystemLibrary.LineTraceSingle` :`Start` (`self.K2_GetActorLocation`) :`End` (`self.K2_GetActorLocation` _asbp_enemy_base) :`TraceChannel` "TraceTypeQuery2" :`DrawDebugType` "ForOneFrame"))
        (`|ExecutionSequence`
          (:`then_0`
            (bind _result (`/Engine/EditorBlueprintResources/StandardMacros.DecrementInt` (`/Game/Blueprints/AI/BP_EnemyBase.health` _asbp_enemy_base))
              (:`  `
                (bind _output_get (set `/Game/Blueprints/AI/BP_EnemyBase.health` _result _asbp_enemy_base))
                (if (> _output_get 0)
                  (`KismetSystemLibrary.Delay` 1.0)
                  (goto _label)
                  (else
                    (`self.K2_DestroyActor` _asbp_enemy_base))))))
          (:`then_1`
            (`|SpawnActorFromClass` "/Game/assets/cannon_tomato/TomatoProjectile.TomatoProjectile_C" (`KismetMathLibrary.MakeTransform` _returnvalue (`KismetMathLibrary.FindLookAtRotation` _returnvalue (`.TraceEnd` (`GameplayStatics.BreakHitResult` _outhit)))) "AlwaysSpawn" "MultiplyWithRoot" null null)
            (`KismetSystemLibrary.Delay` 1.0)
            (goto _label_2)))))
    (else
      (`KismetSystemLibrary.PrintString` "get more ammo"))))

(fn `UserConstructionScript`)