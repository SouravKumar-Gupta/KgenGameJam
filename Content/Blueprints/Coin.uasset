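; Coin is a clickable pickup actor that adds one to the player's currency in the top-down game mode.
; On BeginPlay it caches a cast reference to BP_TopDownGameMode.
; Clicking its Box component increments that mode's Currency and destroys the coin, while Tick spins the Cylinder mesh by a fixed per-frame pitch rotation, independent of delta time.
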(event `self.ReceiveBeginPlay`
  (bind _asbp_top_down_game_mode (cast `/Game/TopDown/Blueprints/BP_TopDownGameMode` (`GameplayStatics.GetGameMode`)))
  (set `self.As BP Top Down Game Mode` _asbp_top_down_game_mode))

(event `self.ReceiveTick`
  (params (DeltaSeconds :type "Float (single-precision)"))
  (`SceneComponent.K2_AddLocalRotation` (`self.Cylinder`) (`KismetMathLibrary.MakeRotator` 0.0 2.0) false false))

(event `self.Box.OnClicked`
  (params (TouchedComponent :type "PrimitiveComponent Object Reference") (ButtonPressed :type "Key Structure"))
  (`/Engine/EditorBlueprintResources/StandardMacros.IncrementInt` (`/Game/TopDown/Blueprints/BP_TopDownGameMode.currency` (`self.As BP Top Down Game Mode`))
    (:`  `
      (`self.K2_DestroyActor`))))

(fn `UserConstructionScript`)